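; BP_Actor is a simple actor that prints its name, health and defense (Nombre, Vida, Defensa) on screen for a long duration at BeginPlay.
; Tick applies a zero local offset, so the actor does not move.
; A local rotation node using VelRotacion is left disconnected, and the Velocidad variable is unused.
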(event EventTick
  (params (DeltaSeconds :type Float%20%28single-precision%29))
  (Transformation|AddActorLocalOffset "0, 0, 0" false false))

(event EventBeginPlay
  (Development|PrintString (Utilities|String|Append "Nombre: 
" (Variables|Propiedades|GetNombre) " 
Vida:" (Utilities|String|ToString(Integer) (Variables|Propiedades|GetVida)) " 
Defensa:" (Utilities|String|ToString(Float) (Variables|Propiedades|GetDefensa))) true true (Variables|Propiedades|GetText%20Color) 3e+01))

(fn ConstructionScript)